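; Enemy character that damages and grabs the player on overlap and dies when struck by a throwable object.
; Player overlap starts a looping damage timer and a delayed grab, which pauses attacks, disables player controls and shows a timed QTE; any end overlap pauses both timers.
; A throwable hit sets IsDead, disables movement and collision, clears both timers and schedules destruction.
; UpdateWalkSpeed exposes a setter for walk speed.
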(event OnComponentHit(CapsuleComponent)
  (params (HitComponent :type Primitive%20Component%20Object%20Reference) (OtherActor :type Actor%20Object%20Reference) (OtherComp :type Primitive%20Component%20Object%20Reference) (NormalImpulse :type Vector :default "0, 0, 0") (Hit :type Hit%20Result%20Structure%20%28by%20ref%29))
  ;[1 1 1] Got hit by the player / dies
  (if (> (Math|Vector|VectorLength NormalImpulse) 0.0)
    (Utilities|Casting|CastToThrowableObjectBP OtherActor)
    (Variables|Default|SetIsDead true)
    (Pawn|Components|CharacterMovement|DisableMovement (Variables|Character|GetCharacterMovement))
    (Collision|SetCollisionEnabled (Variables|Collision|GetCapsuleComponent) "NoCollision")
    (Collision|SetCollisionEnabled (Variables|Default|GetSphere) "NoCollision")
    (Utilities|Time|ClearandInvalidateTimerbyHandle (Variables|Default|GetAttackTimerHandler))
    (Utilities|Time|ClearandInvalidateTimerbyHandle (Variables|Default|GetGrabTimerHandler))
    (Utilities|Time|SetTimerbyEvent (delegate Custom|Destroy%20actor) 15.0)))

(event Custom|AttackPlayer
  ;[1 1 1] Deal damage to the player
  (Default|TakeDamage (stale Collision|EventActorBeginOverlap _output_get) (Variables|Default|GetAttackValue)))

(event Custom|GrabPlayer
  (bind _playercharacter (Variables|Default|GetPlayerCharacter))
  ;[1 1 1] Deal damage to the player
  (Utilities|Time|PauseTimerbyHandle (Variables|Default|GetAttackTimerHandler))
  (Default|DeactivateControls _playercharacter)
  (Default|DisplayQTE _playercharacter "G" "G" true 5.0 self))

(event Custom|Destroy%20actor
  ;[1 1 1] Got hit by the player / dies
  (Actor|DestroyActor))

(event Collision|EventActorBeginOverlap
  (params (OtherActor :type Actor%20Object%20Reference))
  ;[1 1 1] Deal damage to the player
  (bind _asplayer_character_bp (Utilities|Casting|CastToPlayerCharacter_BP OtherActor))
  (bind _output_get (Variables|Default|SetPlayerCharacter _asplayer_character_bp))
  (bind _returnvalue (Utilities|Time|SetTimerbyEvent (delegate Custom|AttackPlayer) (Variables|Default|GetAttackDelay) true))
  (Variables|Default|SetAttackTimerHandler _returnvalue)
  (bind _returnvalue_2 (Utilities|Time|SetTimerbyEvent (delegate Custom|GrabPlayer) (Variables|Default|GetGrabDelay)))
  (Variables|Default|SetGrabTimerHandler _returnvalue_2))

(event Collision|EventActorEndOverlap
  (params (OtherActor :type Actor%20Object%20Reference))
  ;[1 1 1] Deal damage to the player
  (Utilities|Time|PauseTimerbyHandle (Variables|Default|GetAttackTimerHandler))
  (Utilities|Time|PauseTimerbyHandle (Variables|Default|GetGrabTimerHandler)))

(fn ConstructionScript)

(fn UpdateWalkSpeed
  (params (NewWalkSpeed :type Float%20%28double-precision%29))
  (Variables|/Script/Engine.CharacterMovementComponent|SetMaxWalkSpeed (Variables|Character|GetCharacterMovement) NewWalkSpeed))