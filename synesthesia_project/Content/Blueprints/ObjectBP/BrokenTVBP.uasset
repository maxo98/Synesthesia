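; Interactive TV prop whose screen glitches as the player gets closer, toggled on and off through an inherited interaction until broken.
; While on and the player overlaps the range component, Tick maps distance to glitch coefficient, LOD and speed on a dynamic screen material, using maximum values inside the minimum distance.
; A throwable object hit toggles the TV's state, then marks it broken, locking further toggles of screen visibility and range overlap events.
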(event OnComponentBeginOverlap(GlitchCollisionRange)
  (params (OverlappedComponent :type Primitive%20Component%20Object%20Reference) (OtherActor :type Actor%20Object%20Reference) (OtherComp :type Primitive%20Component%20Object%20Reference) (OtherBodyIndex :type Integer) (bFromSweep :type Boolean) (SweepResult :type Hit%20Result%20Structure%20%28by%20ref%29))
  (if (== OtherActor (Game|GetPlayerCharacter 0))
    (Variables|EnemyGlitch|SetInGlitchRange true)))

(event OnComponentEndOverlap(GlitchCollisionRange)
  (params (OverlappedComponent :type Primitive%20Component%20Object%20Reference) (OtherActor :type Actor%20Object%20Reference) (OtherComp :type Primitive%20Component%20Object%20Reference) (OtherBodyIndex :type Integer))
  (if (== (Game|GetPlayerCharacter 0) OtherActor)
    (Variables|EnemyGlitch|SetInGlitchRange false)
    (Rendering|Material|SetScalarParameterValue (Variables|EnemyGlitch|GetGlitchMaterial) "Coefficient" 0.0 :!class /Script/Engine.MaterialInstanceDynamic)))

(event OnComponentHit(StaticMesh)
  (params (HitComponent :type Primitive%20Component%20Object%20Reference) (OtherActor :type Actor%20Object%20Reference) (OtherComp :type Primitive%20Component%20Object%20Reference) (NormalImpulse :type Vector :default "0, 0, 0") (Hit :type Hit%20Result%20Structure%20%28by%20ref%29))
  (Utilities|Casting|CastToThrowableObjectBP OtherActor)
  (CallFunction|ExecuteInteraction)
  (Variables|Default|SetIsBroken true))

(event EventBeginPlay
  (bind _returnvalue (Rendering|Material|CreateDynamicMaterialInstance "/Game/Geometry/Textures/TVScreenGlitchMaterial.TVScreenGlitchMaterial" "None" "None" :!class /Script/Engine.KismetMaterialLibrary))
  (bind _output_get (Variables|EnemyGlitch|SetGlitchMaterial _returnvalue))
  (Rendering|Material|SetMaterial (Variables|Default|GetPlane) 0 _output_get)
  (Rendering|Material|SetScalarParameterValue (Variables|EnemyGlitch|GetGlitchMaterial) "Coefficient" 0.0 :!class /Script/Engine.MaterialInstanceDynamic))

(event EventTick
  (params (DeltaSeconds :type Float%20%28single-precision%29))
  (bind _returnvalue (Transformation|GetActorLocation))
  (bind _returnvalue_2 (Game|GetPlayerCharacter 0))
  (bind _glitchmaterial (Variables|EnemyGlitch|GetGlitchMaterial))
  (bind _glitchmaterial_2 (Variables|EnemyGlitch|GetGlitchMaterial))
  (bind _returnvalue_3 (Transformation|GetActorLocation _returnvalue_2))
  (bind _returnvalue_4 (Math|Vector|Distance(Vector) _returnvalue _returnvalue_3))
  (if (Variables|Default|GetIsOn)
    (if (Variables|EnemyGlitch|GetInGlitchRange)
      (if (<= (Math|Vector|Distance(Vector) (Transformation|GetActorLocation) (Transformation|GetActorLocation (Game|GetPlayerCharacter 0))) (Variables|EnemyGlitch|GetDistanceGlitchMax))
        (if (<= _returnvalue_4 (Variables|EnemyGlitch|GetDistanceGlitchMin))
          (Rendering|Material|SetScalarParameterValue _glitchmaterial_2 "Coefficient" (Variables|EnemyGlitch|GetCoefficientMax) :!class /Script/Engine.MaterialInstanceDynamic)
          (Rendering|Material|SetScalarParameterValue _glitchmaterial_2 "LOD" (Variables|EnemyGlitch|GetLODMax) :!class /Script/Engine.MaterialInstanceDynamic)
          (Rendering|Material|SetScalarParameterValue _glitchmaterial_2 "Vitesse" (Variables|EnemyGlitch|GetVitesseMax) :!class /Script/Engine.MaterialInstanceDynamic)
          (else
            (Rendering|Material|SetScalarParameterValue _glitchmaterial "Coefficient" (Math|Float|MapRangeClamped _returnvalue_4 (Variables|EnemyGlitch|GetDistanceGlitchMin) (Variables|EnemyGlitch|GetDistanceGlitchMax) (Variables|EnemyGlitch|GetCoefficientMax) (Variables|EnemyGlitch|GetCoefficientMin)) :!class /Script/Engine.MaterialInstanceDynamic)
            (Rendering|Material|SetScalarParameterValue _glitchmaterial "LOD" (Math|Float|MapRangeClamped _returnvalue_4 (Variables|EnemyGlitch|GetDistanceGlitchMin) (Variables|EnemyGlitch|GetDistanceGlitchMax) (Variables|EnemyGlitch|GetLODMaxRange) (Variables|EnemyGlitch|GetLODMin)) :!class /Script/Engine.MaterialInstanceDynamic)
            (Rendering|Material|SetScalarParameterValue _glitchmaterial "Vitesse" (Math|Float|MapRangeClamped _returnvalue_4 (Variables|EnemyGlitch|GetDistanceGlitchMin) (Variables|EnemyGlitch|GetDistanceGlitchMax) (Variables|EnemyGlitch|GetVitesseMaxRange) (Variables|EnemyGlitch|GetVitesseMin)) :!class /Script/Engine.MaterialInstanceDynamic)))))))

(fn ConstructionScript
  (|CallParentFunction))

(fn ExecuteInteraction
  (|CallParentFunction)
  (if (not (Variables|Default|GetIsBroken))
    (if (Variables|Default|GetIsOn)
      (bind _output_get (Variables|Default|SetIsOn false))
      (Rendering|SetVisibility (Variables|Default|GetPlane) _output_get false)
      (Variables|/Script/Engine.PrimitiveComponent|SetbGenerateOverlapEvents (Variables|Default|GetGlitchCollisionRange) _output_get)
      (else
        (bind _output_get_2 (Variables|Default|SetIsOn true))
        (Rendering|SetVisibility (Variables|Default|GetPlane) _output_get_2 false)
        (Variables|/Script/Engine.PrimitiveComponent|SetbGenerateOverlapEvents (Variables|Default|GetGlitchCollisionRange) _output_get_2)))))