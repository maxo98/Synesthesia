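; ButtonBP is an interactable button object that toggles its look each time it is used.
; It overrides Execute Interaction, calls the parent version, then swaps the first material slot of its static mesh between BaseMaterial and BaseMaterial_2.
; The currently applied material serves as the toggle state, with no separate boolean.
; The event graph and construction script add no logic of their own.
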(event EventBeginPlay)

(event Collision|EventActorBeginOverlap
  (params (OtherActor :type Actor%20Object%20Reference))
  (|CallParentFunction OtherActor) ; This node is disabled and will not be called.\nDrag off pins to build functionality.
)

(event EventTick
  (params (DeltaSeconds :type Float%20%28single-precision%29)))

(fn ConstructionScript
  (|CallParentFunction))

(fn ExecuteInteraction
  (bind _staticmesh (Variables|Default|GetStaticMesh))
  (|CallParentFunction)
  (if (== (Utilities|Array|Get(acopy) (Rendering|Material|GetMaterials (Variables|Default|GetStaticMesh))) "/Game/FirstPerson/Meshes/BaseMaterial_2.BaseMaterial_2")
    (Rendering|Material|SetMaterial _staticmesh 0 "/Game/FirstPerson/Meshes/BaseMaterial.BaseMaterial")
    (else
      (Rendering|Material|SetMaterial _staticmesh 0 "/Game/FirstPerson/Meshes/BaseMaterial_2.BaseMaterial_2"))))