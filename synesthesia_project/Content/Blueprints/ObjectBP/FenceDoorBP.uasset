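; Interactable fence door that is locked behind a keypad code, using a keypad UI taken from its widget component.
; CheckCode compares entered codes with the correct one, then unlocks and opens the door or signals a wrong code, clearing the entry.
; Interacting toggles the door when unlocked, or shows the wrong-code response when locked.
; A timeline drives the mesh's yaw or roll swing through RInterpTo and reverses to close.
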(event Custom|CloseDoor
  (bind _value (Timeline|OpenCloseDoorTimeline Reverse)
    (:Update
      (Transformation|SetRelativeRotation (Variables|Default|GetDoorMesh) (Math|Interpolation|RInterpTo "0, 0, 0" "0,-90.000000, 0" _value 2.0) false false))))

(event Custom|OpenDoor
  (bind _value (Timeline|OpenCloseDoorTimeline Play)
    (:Update
      (Transformation|SetRelativeRotation (Variables|Default|GetDoorMesh) (Math|Interpolation|RInterpTo "0, 0, 0" "0,-90.000000, 0" _value 2.0) false false))))

(event EventBeginPlay
  (bind _askey_pad_ui (Utilities|Casting|CastToKeyPadUI (UserInterface|GetUserWidgetObject (Variables|Default|GetKeyPadWidget))))
  (bind _output_get (Variables|Default|SetKeyPadUI _askey_pad_ui))
  (EventDispatchers|BindEventtoCodeEntered _output_get (EventDispatchers|CreateEvent :!event CheckCode)))

(event Collision|EventActorBeginOverlap
  (params (OtherActor :type Actor%20Object%20Reference))
  (|CallParentFunction OtherActor))

(fn ConstructionScript
  (|CallParentFunction))

(fn ExecuteInteraction
  (|CallParentFunction)
  (if (Variables|Default|GetIsLocked)
    (Default|WrongCode (Variables|Default|GetKeyPadUI))
    (elif (Variables|Default|GetIsOpen)
      (CallFunction|CloseDoor)
      (Variables|Default|SetIsOpen false)
      (else
        (CallFunction|OpenDoor)
        (Variables|Default|SetIsOpen true)))))

(fn CheckCode
  (params (Code :type String) (KeyPad :type Key%20Pad%20UI%20Object%20Reference))
  (if (Utilities|Enum|Equal(Enum) Code (Variables|Default|GetCorrectCode))
    (Variables|Default|SetIsLocked false)
    (Default|CorrectCode KeyPad)
    (CallFunction|OpenDoor)
    (Variables|/Game/UI/KeyPadUI/KeyPadUI.KeyPadUI_C|SetCurrentCode KeyPad "")
    (else
      (Default|WrongCode KeyPad)
      (Variables|/Game/UI/KeyPadUI/KeyPadUI.KeyPadUI_C|SetCurrentCode KeyPad ""))))