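; Subway light lever, a child interactable Blueprint that switches a group of spot lights and their fixture meshes when used.
; Its ExecuteInteraction override calls the parent, branches on LightOn, then sets each spot light's visibility and swaps fixture materials between on and off, in nested loops.
; LightOn becomes true inside the inner turn-on loop, but its reset to false is unconnected, so once it is set, later interactions only switch lights off.
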(event Collision|EventActorBeginOverlap
  (params (OtherActor :type Actor%20Object%20Reference))
  (|CallParentFunction OtherActor) ; This node is disabled and will not be called.\nDrag off pins to build functionality.
)

(fn ConstructionScript
  (|CallParentFunction))

(fn ExecuteInteraction
  (bind _spotlights (Variables|Default|GetSpotLights))
  (bind _physicallight (Variables|Default|GetPhysicalLight))
  (|CallParentFunction)
  (if (Variables|Default|GetLightOn?)
    (for _array_element _spotlights
      (Rendering|SetVisibility (Variables|/Script/Engine.SpotLight|GetSpotLightComponent _array_element) false true)
      (for _array_element_2 _physicallight
        (Rendering|Material|SetMaterial (Variables|/Script/Engine.StaticMeshActor|GetStaticMeshComponent _array_element_2) 0 "/Game/Underground/Materials/Instances/Mi_Lights_Off.Mi_Lights_Off")))
    (else
      (for _array_element_3 _spotlights
        (Rendering|SetVisibility (Variables|/Script/Engine.SpotLight|GetSpotLightComponent _array_element_3) true true)
        (for _array_element_4 _physicallight
          (Rendering|Material|SetMaterial (Variables|/Script/Engine.StaticMeshActor|GetStaticMeshComponent _array_element_4) 0 "/Game/Underground/Materials/Instances/Mi_Lights_On.Mi_Lights_On")
          (Variables|Default|SetLightOn? true))))))