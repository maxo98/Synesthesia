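; AI controller for the monster that starts BT_Monster on BeginPlay and feeds it what its perception component detects.
; Perception updates are routed to HandleSense, which switches on the sense class's display name and handles only sight.
; Sight sets IsInvestigating to whether the stimulus was sensed, and stores the seen actor in TagetLocationActor on success.
; Losing sight clears the flag but leaves the last stored actor in the Blackboard.
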(event OnTargetPerceptionUpdated(AIPerception)
  (params (Actor :type Actor%20Object%20Reference) (Stimulus :type AI%20Stimulus%20Structure))
  (bind _returnvalue (Class|AIPerceptionSystem|GetSenseClassforStimulus Stimulus))
  (CallFunction|HandleSense (Utilities|GetClassDisplayName _returnvalue) Stimulus Actor))

(event EventBeginPlay
  (AI|RunBehaviorTree "/Game/Blueprints/monsterBP/BT_Monster.BT_Monster"))

(fn ConstructionScript)

(fn HandleSense
  (params (Selection :type String) (Stimulus :type AI%20Stimulus%20Structure) (SensedActor :type Actor%20Object%20Reference))
  (switch string Selection
    (:AiSense_Sight
      (AI|Components|Blackboard|SetValueasBool (Variables|Default|GetBlackboard) (Utilities|Name|MakeLiteralName "IsInvestigating") (.bsuccessfullysensed Stimulus))
      (if (.bsuccessfullysensed Stimulus)
        (AI|Components|Blackboard|SetValueasObject (Variables|Default|GetBlackboard) (Utilities|Name|MakeLiteralName "TagetLocationActor") SensedActor)))))